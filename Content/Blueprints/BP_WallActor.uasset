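; BP_WallActor is a construction-time wall builder that generates walls along an editable spline, with configurable height and materials.
; The Construction Script can reset the spline to a default square, using clamped points with near-zero tangents for sharp corners.
; On reset or when UpdateSplineMeshes is set, it adds spline mesh wall segments with per-side materials, then builds a procedural cap mesh from planar vertices.
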(fn `CreateDefaultSplineShape`
  (bind _splinecomponent (`self.SplineComponent`))
  (bind _splinecomponent_2 (`self.SplineComponent`))
  (bind _returnvalue (/ (`self.DefaultSize`) 2.0))
  (bind _returnvalue_2 (* _returnvalue -1.0))
  (`SplineComponent.ClearSplinePoints` _splinecomponent true)
  (`SplineComponent.AddSplinePoint` _splinecomponent (`KismetMathLibrary.MakeVector` _returnvalue _returnvalue) "Local" true)
  (`SplineComponent.AddSplinePoint` _splinecomponent (`KismetMathLibrary.MakeVector` _returnvalue_2 _returnvalue) "Local" true)
  (`SplineComponent.AddSplinePoint` _splinecomponent (`KismetMathLibrary.MakeVector` _returnvalue_2 _returnvalue_2) "Local" true)
  (`SplineComponent.AddSplinePoint` _splinecomponent (`KismetMathLibrary.MakeVector` _returnvalue _returnvalue_2) "Local" true)
  (for _index (range (`SplineComponent.GetNumberOfSplinePoints` (`self.SplineComponent`)))
    (`SplineComponent.SetSplinePointType` _splinecomponent_2 _index "CurveClamped" true)
    (bind (_returnvalue_x _returnvalue_y _returnvalue_z) (`KismetMathLibrary.BreakVector` (`SplineComponent.GetTangentAtSplinePoint` _splinecomponent_2 _index "Local")))
    (`SplineComponent.SetTangentAtSplinePoint` _splinecomponent_2 _index (`KismetMathLibrary.MakeVector` 0.0001 0.0001 _returnvalue_z) "Local" true)))

(fn `UserConstructionScript`
  (if (`self.bResetSplineToDefault`)
    (`self.CreateDefaultSplineShape`)
    (bind (_outsplinepointvertices _outsidematerials) (`/Game/Blueprints/SplineActors/SplineActorFunctionLibrary.AddSplineMeshComponents` null self (`self.Height`) (`self.SideMaterials`) (`self.NumberTextures`) (`self.SplineWallMesh`) (`self.UseMaterialZeroForAllWalls`) :!label _label))
    (set `self.Spline Point Vertices` _outsplinepointvertices)
    (set `self.SideMaterials` _outsidematerials)
    (`/Game/Blueprints/SplineActors/SplineActorFunctionLibrary.CreateProceduralMeshForPlanarVertices` (`self.Height`) (`self.Cap Material`) (`self.ProceduralMesh`) null (`self.Number of Spline sub-divisions`))
    (elif (`self.bUpdateSplineMeshes`)
      (goto _label))))